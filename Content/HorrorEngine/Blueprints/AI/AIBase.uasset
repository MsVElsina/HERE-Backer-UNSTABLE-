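; Base AI character for HorrorEngine, providing walk and chase speeds, health, and death or stun handling.
; Head and chest hitbox overlaps with tagged actors apply separate damage values, gated by a Damageable enum.
; At zero health it either collapses and is destroyed, or crouches stunned while healing to its starting health.
; Ghost variants hide their mesh from the player via owner-no-see; hit reactions are empty stubs.
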(event `self.ReceiveBeginPlay`
  (`|ExecutionSequence`
    (:`then_0`
      (set `self.AnimBP` (cast `/Game/Mannequin/Animations/ThirdPerson_AnimBP` (`SkeletalMeshComponent.GetAnimInstance` (`self.Mesh`)) :!pure true)))
    (:`then_1`
      (`self.SetOwner` (`GameplayStatics.GetPlayerPawn` 0))
      (if (`self.Ghost`)
        (`PrimitiveComponent.SetOwnerNoSee` (`self.Mesh`) true)))))

(event `Run`
  ;[1 1 1] Movement
  (set `CharacterMovementComponent.MaxWalkSpeed` (`self.ChaseSpeed`) (`self.CharacterMovement`)))

(event `Walk`
  ;[1 1 1] Movement
  (set `CharacterMovementComponent.MaxWalkSpeed` (`self.WalkSpeed`) (`self.CharacterMovement`)))

(event `Damage`
  (params (DamageAmount :type "Float (double-precision)"))
  ;[1 1 1] Damage
  (if (`|EnumInequality` (`self.Damageable`) "NewEnumerator2")
    (bind _output_get (set `self.Health` (- (`self.Health`) DamageAmount)))
    (`KismetSystemLibrary.PrintString` (`KismetStringLibrary.Conv_DoubleToString` _output_get))
    (`self.CheckHealth`)))

(event `CheckHealth`
  ;[1 1 1] Health
  (if (< (`self.Health`) 1.0)
    (`self.No health`)
    (`KismetSystemLibrary.PrintString` "I am become Died")
    (else
      (`self.React`))))

(event `No health`
  ;[1 1 1] No Health
  (if (`|EnumInequality` (`self.Damageable`) "NewEnumerator1")
    (`SkeletalMeshComponent.PlayAnimation` (`self.Mesh`) "/Game/HorrorEngine/Blueprints/AI/Stand_To_Prone1.Stand_To_Prone1" false)
    (`ActorComponent.Deactivate` (`self.CharacterMovement`))
    (`PrimitiveComponent.SetCollisionEnabled` (`self.CapsuleComponent`) "NoCollision")
    (`KismetSystemLibrary.Delay` 3.0)
    (`self.K2_DestroyActor`)
    (else
      (`self.Stunned`))))

(event `Stunned`
  (bind _health (`self.Health`))
  ;[1 1 1] Stunned State
  (`ActorComponent.Deactivate` (`self.CharacterMovement`))
  (`SkeletalMeshComponent.PlayAnimation` (`self.Mesh`) "/Game/HorrorEngine/Blueprints/AI/Crouch.Crouch" true)
  (if (< (`self.Health`) (`self.MaxHealth`)) :!label _label
    (`KismetSystemLibrary.PrintString` (`KismetStringLibrary.Conv_DoubleToString` _health))
    (set `self.Health` (+ _health 25.0))
    (`KismetSystemLibrary.PrintString` "Healing")
    (`KismetSystemLibrary.Delay` 2.0)
    (goto _label)
    (else
      (`SkeletalMeshComponent.SetAnimationMode` (`self.Mesh`) "AnimationBlueprint")
      (`ActorComponent.Activate` (`self.CharacterMovement`) false))))

(event `React`
  ;[1 1 1] Hit React
)

(event `self.ChestHitbox.OnComponentBeginOverlap`
  (params (OverlappedComponent :type "PrimitiveComponent Object Reference") (OtherActor :type "Actor Object Reference") (OtherComp :type "PrimitiveComponent Object Reference") (OtherBodyIndex :type Integer) (bFromSweep :type Boolean) (SweepResult :type "HitResult Structure (by ref)"))
  ;[1 1 1] Chest Hit
  (if (`self.ActorHasTag` OtherActor "GetFucked")
    (`KismetSystemLibrary.PrintString` "Have at you")
    (`self.Damage` (`self.ChestHitVal`))))

(event `self.HeadHitbox.OnComponentBeginOverlap`
  (params (OverlappedComponent :type "PrimitiveComponent Object Reference") (OtherActor :type "Actor Object Reference") (OtherComp :type "PrimitiveComponent Object Reference") (OtherBodyIndex :type Integer) (bFromSweep :type Boolean) (SweepResult :type "HitResult Structure (by ref)"))
  ;[1 1 1] Head Hit
  (if (`self.ActorHasTag` OtherActor "GetFucked")
    (`KismetSystemLibrary.PrintString` "Dommed")
    (`self.Damage` (`self.HeadHitVal`))))

(fn `UserConstructionScript`
  (`|ExecutionSequence`
    (:`then_0`
      (set `self.MaxHealth` (`self.Health`))
      (if (`|EnumInequality` (`self.Temperment`) "NewEnumerator2")
        _))))