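; Base AI controller for AIBase pawns that runs the Base_BT behavior tree to drive patrolling and player detection.
; On BeginPlay, patrolling pawns copy their route loop and direction settings, plus the player character, into the Blackboard.
; Perception updates set CanSeePlayer for any sensed actor, skipped for one temperament.
; GetNextPoint writes the current patrol point to the Blackboard, then advances the index forward with wraparound.
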(event `self.ReceiveBeginPlay`
  (bind _returnvalue (`AIBlueprintHelperLibrary.GetBlackboard` null))
  (`self.RunBehaviorTree` "/Game/HorrorEngine/Blueprints/AI/Base_BT.Base_BT")
  (bind _asaibase (cast `/Game/HorrorEngine/Blueprints/AI/AIBase` (`self.K2_GetPawn`)))
  (bind _output_get (set `self.BasicPawn` _asaibase))
  (bind _patrols (`/Game/HorrorEngine/Blueprints/AI/AIBase.Patrols` _output_get))
  (if _patrols
    (`BlackboardComponent.SetValueAsBool` (`AIBlueprintHelperLibrary.GetBlackboard` null) "Patrols" _patrols)
    (`BlackboardComponent.SetValueAsBool` _returnvalue "RouteLoops" (`/Game/HorrorEngine/Blueprints/AI/AIBase.LoopPath` _output_get))
    (if (`|EnumEquality` (`/Game/HorrorEngine/Blueprints/AI/AIBase.Direction` _output_get) "NewEnumerator0")
      (`BlackboardComponent.SetValueAsInt` _returnvalue "Direction" 1)
      (`KismetSystemLibrary.PrintString` "Go Forward")
      (else
        (`BlackboardComponent.SetValueAsInt` _returnvalue "Direction" -1)
        (`KismetSystemLibrary.PrintString` "Go Backward")))
    (`BlackboardComponent.SetValueAsObject` (`AIBlueprintHelperLibrary.GetBlackboard` null) "PlayerObject" (`GameplayStatics.GetPlayerCharacter` 0))))

(event `self.AIPerception.OnTargetPerceptionUpdated`
  (params (Actor :type "Actor Object Reference") (Stimulus :type "AIStimulus Structure"))
  (if (`|EnumInequality` (`/Game/HorrorEngine/Blueprints/AI/AIBase.Temperment` (`self.BasicPawn`)) "NewEnumerator0")
    (`BlackboardComponent.SetValueAsBool` (`AIBlueprintHelperLibrary.GetBlackboard` null) "CanSeePlayer" (`.bSuccessfullySensed` (break `AIStimulus` Stimulus)))))

(event `GetNextPoint`
  (bind _patrolpoints (`/Game/HorrorEngine/Blueprints/AI/PatrolPath.PatrolPoints` (`/Game/HorrorEngine/Blueprints/AI/AIBase.PatrolPath` (`self.BasicPawn`))))
  ;[1 1 1] Get next Target in array
  (`BlackboardComponent.SetValueAsObject` (`AIBlueprintHelperLibrary.GetBlackboard` null) "TargetPointKey" (`|GetArrayItem` _patrolpoints (`self.CurrentArrayIndex`)))
  (if (>= (`self.CurrentArrayIndex`) (- (`KismetArrayLibrary.Array_Length` _patrolpoints) 1))
    (set `self.CurrentArrayIndex` 0)
    (else
      (set `self.CurrentArrayIndex` (+ (`self.CurrentArrayIndex`) 1)))))

(fn `UserConstructionScript`)